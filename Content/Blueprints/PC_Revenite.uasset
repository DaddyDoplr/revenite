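; PC_Revenite is a player controller that toggles game pause and forwards gamepad D-pad presses.
; Pausing creates the Anomaly pause menu, shows the cursor near the bottom center of the screen and switches to Game and UI input.
; Unpausing removes all widgets, including that menu, hides the cursor and restores game-only input.
; D-pad up and down fire the Up and Down calls.
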(event `InputAction|Pause` :paused true
  (params (Key :type "Key Structure"))
  (bind (_sizex _sizey) (`self.GetViewportSize`))
  (:`Pressed`
    (`GameplayStatics.SetGamePaused` (not (`GameplayStatics.IsGamePaused`)))
    (if (`GameplayStatics.IsGamePaused`)
      ;[1 1 1] Pause Widget Currently set to Anomaly Pause Menu
      (bind _returnvalue (`|CreateWidget` "/Game/UI/PauseMenu/UI_PauseMenuAnomaly.UI_PauseMenuAnomaly_C"))
      (`UserWidget.AddToViewport` _returnvalue 0)
      (set `self.bShowMouseCursor` true)
      (`WidgetBlueprintLibrary.SetInputMode_GameAndUIEx` self _returnvalue "LockAlways" false)
      (`self.SetMouseLocation` (/ _sizex 2) (- _sizey 200))
      (else
        (`Widget.RemoveFromParent` _returnvalue)
        (`WidgetLayoutLibrary.RemoveAllWidgets`)
        (set `self.bShowMouseCursor` false)
        (`WidgetBlueprintLibrary.SetInputMode_GameOnly` self)))))

(event `Key|Gamepad_DPad_Up`
  (params (Key :type "Key Structure"))
  (:`Pressed`
    (`self.Up`)))

(event `Key|Gamepad_DPad_Down`
  (params (Key :type "Key Structure"))
  (:`Pressed`
    (`self.Down`)))

(fn `UserConstructionScript`)