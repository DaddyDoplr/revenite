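; Player controller Blueprint that toggles the pause menu when the Pause input is pressed.
; Pausing creates a new UI_PauseMenu widget, adds it to the viewport, shows the cursor centered on screen and focuses the menu in Game and UI input mode.
; Unpausing removes the widget, hides the cursor and restores game-only input.
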(event `InputAction|Pause` :paused true
  (params (Key :type "Key Structure"))
  (bind (_sizex _sizey) (`self.GetViewportSize`))
  (:`Pressed`
    (`GameplayStatics.SetGamePaused` (not (`GameplayStatics.IsGamePaused`)))
    (if (`GameplayStatics.IsGamePaused`)
      (bind _returnvalue (`|CreateWidget` "/Game/UI/PauseMenu/UI_PauseMenu.UI_PauseMenu_C"))
      (`UserWidget.AddToViewport` _returnvalue 0)
      (set `self.bShowMouseCursor` true)
      (`WidgetBlueprintLibrary.SetInputMode_GameAndUIEx` self _returnvalue "DoNotLock" false)
      (`self.SetMouseLocation` (/ _sizex 2) (/ _sizey 2))
      (else
        (`Widget.RemoveFromParent` _returnvalue)
        (set `self.bShowMouseCursor` false)
        (`WidgetBlueprintLibrary.SetInputMode_GameOnly` self)))))

(fn `UserConstructionScript`)