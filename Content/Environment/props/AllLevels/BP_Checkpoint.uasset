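; BP_Checkpoint is a one-time checkpoint prop that plays feedback when hit, then removes itself.
; CheckpointHit fires OnCollide and returns the root's location and rotation to the caller, with no overlap detection in this Blueprint.
; OnCollide shows a checkpoint text widget, plays a sound and spawns a pickup particle.
; Chained timelines multiply current mesh scale, then particle scale and light intensity, compounding each update before destroying the actor.
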(event `OnCollide`
  (bind _checkpoint_mesh (`self.Checkpoint_Mesh`))
  (bind _pt_checkpoint (`self.PT_Checkpoint`))
  (bind _pointlight (`self.PointLight`))
  (bind (_returnvalue_location _returnvalue_rotation) (`KismetMathLibrary.BreakTransform` (`SceneComponent.K2_GetComponentToWorld` (`self.Root`))))
  (bind _returnvalue (`|CreateWidget` "/Game/UI/UI_CheckpointText.UI_CheckpointText_C"))
  (`UserWidget.AddToViewport` _returnvalue 0)
  (`GameplayStatics.SpawnSound2D` "/Game/UI/SFX/SFX_-_Menu_Scroll_W_REVERB.SFX_-_Menu_Scroll_W_REVERB" 1.0 1.0 0.0 null)
  (`GameplayStatics.SpawnEmitterAtLocation` "/Game/Pickups/PT_Pickup.PT_Pickup" _returnvalue_location _returnvalue_rotation)
  (bind (_direction _scaler) (`Timeline|scaleMesh` :!via `PlayFromStart`)
    (:`Update`
      (`SceneComponent.SetWorldScale3D` _checkpoint_mesh (* (`SceneComponent.K2_GetComponentScale` _checkpoint_mesh) _scaler)))
    (:`Finished`
      (bind (_direction_2 _scaler_2) (`Timeline|scaleLights` :!via `PlayFromStart`)
        (:`Update`
          (`SceneComponent.SetWorldScale3D` _pt_checkpoint (* (`SceneComponent.K2_GetComponentScale` _pt_checkpoint) _scaler_2))
          (`LightComponent.SetIntensity` _pointlight (* _scaler_2 (`LightComponentBase.Intensity` _pointlight))))
        (:`Finished`
          (`self.K2_DestroyActor`))))))

(fn `checkpointHit`
  (returns (outLoc :type "Vector Structure") (outRot :type "Rotator Structure"))
  (`self.OnCollide`)
  (bind (_outloc _outrot) (`self.setTransform`))
  (return _outloc _outrot))

(fn `setTransform`
  (returns (outLoc :type "Vector Structure") (outRot :type "Rotator Structure"))
  (bind (_returnvalue_location _returnvalue_rotation) (`KismetMathLibrary.BreakTransform` (`SceneComponent.K2_GetComponentToWorld` (`self.Root`))))
  (return _returnvalue_location _returnvalue_rotation))

(fn `UserConstructionScript`)